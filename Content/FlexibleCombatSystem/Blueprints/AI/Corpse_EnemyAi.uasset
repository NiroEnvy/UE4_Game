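; Corpse enemy AI for the Flexible Combat System, supplying corpse-specific animations and stats for each weapon style.
; SetupWeapon maps the equipped weapon enum (fists, axe and shield, two-handed or dual-wield) to a WeaponInfo struct, then unpacks it into damage, combo, draw and sheathe variables.
; It caches the weapon type and resets the enum so armed animations wait until combat.
; The event graph holds no active logic.
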(fn `SetupWeapon`
  (bind _equippedweaponenum (`self.EquippedWeaponEnum`))
  (bind (_equippedweaponclass _equippedweaponobject _weapontype _weaponbasedamage _numberofcomboattacks _comboattackanim1 _comboattackanim2 _comboattackanim3 _comboattackanim4 _drawweaponanim _sheatheweaponanim) (break `/Game/FlexibleCombatSystem/Structs/S_WeaponStats` (`self.WeaponInfo`)))
  (if (`|EnumEquality` _equippedweaponenum "NewEnumerator2")
    ;[1 1 1] Fist Weapon Info
    (set `self.WeaponInfo` (make `/Game/FlexibleCombatSystem/Structs/S_WeaponStats` "/Game/FlexibleCombatSystem/Blueprints/Weapons/AI/BP_AI_Fists.BP_AI_Fists_C" null "NewEnumerator2" 4.0 4 "/Game/CityofBrass_Enemies/Meshes/Enemy/Corpse/animation/Fists/Corpse_M_Fists_AttackA.Corpse_M_Fists_AttackA" "/Game/CityofBrass_Enemies/Meshes/Enemy/Corpse/animation/Fists/Corpse_M_Fists_AttackB.Corpse_M_Fists_AttackB" "/Game/CityofBrass_Enemies/Meshes/Enemy/Corpse/animation/Fists/Corpse_M_Fists_AttackC.Corpse_M_Fists_AttackC" "/Game/CityofBrass_Enemies/Meshes/Enemy/Corpse/animation/Fists/Corpse_M_Fists_AttackD.Corpse_M_Fists_AttackD"))
    ;[1 1 1] Depending What Weapon Equipped, Sets Weapon Info Here
    (set `self.WeaponBaseDamage` _weaponbasedamage :!label _label)
    (set `self.NumberOfWeaponAttacks` _numberofcomboattacks)
    (set `self.ComboAttack1Anim` _comboattackanim1)
    (set `self.ComboAttack2Anim` _comboattackanim2)
    (set `self.ComboAttack3Anim` _comboattackanim3)
    (set `self.ComboAttack4Anim` _comboattackanim4)
    (set `self.DrawWeaponAnim` _drawweaponanim)
    (set `self.SheatheWeaponAnim` _sheatheweaponanim)
    ;;[1 1 1] We create a reference to the weapon and then set the weapon to empty. This is because the "EquippedWeapon" changes the outputted animation. We don't want the character to be playing weapon attack animations until he draws his weapon and is in combat. So for now we create a reference and clear it (until the AI is in combat)
    (set `self.EquippedWeaponRef` _weapontype)
    (set `self.EquippedWeaponEnum` "NewEnumerator4")
    (elif (`|EnumEquality` _equippedweaponenum "NewEnumerator0")
      ;[1 1 1] Axe And Shield Weapon Info
      (set `self.WeaponInfo` (make `/Game/FlexibleCombatSystem/Structs/S_WeaponStats` "/Game/FlexibleCombatSystem/Blueprints/Weapons/AI/BP_AI_AxeAndShield.BP_AI_AxeAndShield_C" null "NewEnumerator0" 25.0 4 "/Game/CityofBrass_Enemies/Meshes/Enemy/Corpse/animation/axeAndShield/Corpse_M_AxeAndShield_AttackA.Corpse_M_AxeAndShield_AttackA" "/Game/CityofBrass_Enemies/Meshes/Enemy/Corpse/animation/axeAndShield/Corpse_M_AxeAndShield_AttackB.Corpse_M_AxeAndShield_AttackB" "/Game/CityofBrass_Enemies/Meshes/Enemy/Corpse/animation/axeAndShield/Corpse_M_AxeAndShield_Attack_C.Corpse_M_AxeAndShield_Attack_C" "/Game/CityofBrass_Enemies/Meshes/Enemy/Corpse/animation/axeAndShield/Corpse_M_AxeAndShield_AttackD.Corpse_M_AxeAndShield_AttackD" "/Game/CityofBrass_Enemies/Meshes/Enemy/Corpse/animation/axeAndShield/Corpse_M_AxeAndShield_DrawWeapon.Corpse_M_AxeAndShield_DrawWeapon" "/Game/CityofBrass_Enemies/Meshes/Enemy/Corpse/animation/axeAndShield/Corpse_M_AxeAndShield_SheatheWeapon.Corpse_M_AxeAndShield_SheatheWeapon"))
      (goto _label)
      (elif (`|EnumEquality` _equippedweaponenum "NewEnumerator1")
        ;[1 1 1] 2H Weapon Info
        (set `self.WeaponInfo` (make `/Game/FlexibleCombatSystem/Structs/S_WeaponStats` "/Game/FlexibleCombatSystem/Blueprints/Weapons/AI/BP_AI_2HWeapon.BP_AI_2HWeapon_C" null "NewEnumerator1" 35.0 4 "/Game/CityofBrass_Enemies/Meshes/Enemy/Corpse/animation/2H/Corpse_M_2H_AttackA.Corpse_M_2H_AttackA" "/Game/CityofBrass_Enemies/Meshes/Enemy/Corpse/animation/2H/Corpse_M_2H_AttackD.Corpse_M_2H_AttackD" "/Game/CityofBrass_Enemies/Meshes/Enemy/Corpse/animation/2H/Corpse_M_2H_AttackC.Corpse_M_2H_AttackC" "/Game/CityofBrass_Enemies/Meshes/Enemy/Corpse/animation/2H/Corpse_M_2H_AttackD.Corpse_M_2H_AttackD" "/Game/CityofBrass_Enemies/Meshes/Enemy/Corpse/animation/2H/Corpse_M_2H_DrawWeapon.Corpse_M_2H_DrawWeapon" "/Game/CityofBrass_Enemies/Meshes/Enemy/Corpse/animation/2H/Corpse_M_2H_SheatheWeapon.Corpse_M_2H_SheatheWeapon"))
        (goto _label)
        (elif (`|EnumEquality` _equippedweaponenum "NewEnumerator3")
          ;[1 1 1] Dual-Wield Weapon Info
          (set `self.WeaponInfo` (make `/Game/FlexibleCombatSystem/Structs/S_WeaponStats` "/Game/FlexibleCombatSystem/Blueprints/Weapons/AI/BP_AI_DualWield.BP_AI_DualWield_C" null "NewEnumerator3" 15.0 4 "/Game/CityofBrass_Enemies/Meshes/Enemy/Corpse/animation/DualDaggers/Corpse_M_DualWield_AttackA.Corpse_M_DualWield_AttackA" "/Game/CityofBrass_Enemies/Meshes/Enemy/Corpse/animation/DualDaggers/Corpse_M_DualWield_AttackB.Corpse_M_DualWield_AttackB" "/Game/CityofBrass_Enemies/Meshes/Enemy/Corpse/animation/DualDaggers/Corpse_M_DualWield_AttackC.Corpse_M_DualWield_AttackC" "/Game/CityofBrass_Enemies/Meshes/Enemy/Corpse/animation/DualDaggers/Corpse_M_DualWield_AttackD.Corpse_M_DualWield_AttackD" "/Game/CityofBrass_Enemies/Meshes/Enemy/Corpse/animation/DualDaggers/Corpse_M_DualWield_DrawWeapon.Corpse_M_DualWield_DrawWeapon" "/Game/CityofBrass_Enemies/Meshes/Enemy/Corpse/animation/DualDaggers/Corpse_M_DualWield_SheatheWeapon.Corpse_M_DualWield_SheatheWeapon"))
          (goto _label))))))

(fn `UserConstructionScript`
  (`parent.UserConstructionScript`))