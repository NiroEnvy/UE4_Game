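; Trigger box that fades the screen out and then reveals text when the player character enters it.
; On overlap, the Fade Screen graph adds a new WB_Fader widget to the viewport and runs a Timeline that raises its image's tint alpha from clear toward opaque black.
; When the Timeline finishes, the widget is returned to the event graph, which makes its TextBlock visible.
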(event `self.ReceiveActorBeginOverlap`
  (params (OtherActor :type "Actor Object Reference"))
  (cast `/Game/FlexibleCombatSystem/Blueprints/BP_PlayerCharacter` OtherActor)
  (bind _returnvalue (`|CreateWidget` "/Game/MyContent/Widgets/WB_Fader.WB_Fader_C"))
  (`UserWidget.AddToViewport` _returnvalue 0)
  (bind (_direction _newtrack_0) (`Timeline|Timeline`)
    (:`Update`
      (`Image.SetBrushTintColor` (`/Game/MyContent/Widgets/WB_Fader.Image` _returnvalue) (make `SlateColor` (make `LinearColor` 0.0 0.0 0.0 (`KismetMathLibrary.Lerp` 0.0 1.0 _newtrack_0)))))
    (:`Finished`
      ;[1 1 1] Show text
      (`Widget.SetVisibility` (`/Game/MyContent/Widgets/WB_Fader.TextBlock` _returnvalue) "Visible"))))

(fn `UserConstructionScript`)