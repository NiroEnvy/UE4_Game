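; BP_TrainingTrigger is a trigger actor that shows a training tip when the player character overlaps it.
; On BeginPlay it reuses an existing top-level WB_TrainTip widget or creates one.
; Player overlap adds the widget to the viewport and passes it TextForTip to display.
; Tick repeats this whenever a player is inside and the widget is off screen, intended to cover spawning inside the trigger.
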(event `self.ReceiveBeginPlay`
  ;[1 1 1] Create or set wb on level
  (`|ExecutionSequence`
    (:`then_0`
      (bind _foundwidgets (`WidgetBlueprintLibrary.GetAllWidgetsOfClass` "/Game/MyContent/Widgets/WB_TrainTip.WB_TrainTip_C"))
      (if (`KismetArrayLibrary.Array_IsEmpty` _foundwidgets)
        (bind _returnvalue (`|CreateWidget` "/Game/MyContent/Widgets/WB_TrainTip.WB_TrainTip_C"))
        (set `self.TipWidget` _returnvalue)
        (else
          (set `self.TipWidget` (`|GetArrayItem` _foundwidgets)))))))

(event `self.ReceiveActorBeginOverlap`
  (params (OtherActor :type "Actor Object Reference"))
  (bind _tipwidget (`self.TipWidget`))
  ;[1 1 1] Update text
  (cast `/Game/FlexibleCombatSystem/Blueprints/BP_PlayerCharacter` OtherActor)
  (`UserWidget.AddToViewport` _tipwidget 0 :!label _label)
  (`/Game/MyContent/Widgets/WB_TrainTip.Update and show text` _tipwidget (`self.Text for tip`)))

(event `self.ReceiveTick`
  (params (DeltaSeconds :type "Float (single-precision)"))
  ;[1 1 1] Check if we spawn inside trigger
  (if (and (== (`KismetArrayLibrary.Array_IsEmpty` (`self.GetOverlappingActors` "/Game/FlexibleCombatSystem/Blueprints/BP_PlayerCharacter.BP_PlayerCharacter_C")) false) (== (`Widget.IsInViewport` (`self.TipWidget`)) false))
    (goto _label)))

(fn `UserConstructionScript`)