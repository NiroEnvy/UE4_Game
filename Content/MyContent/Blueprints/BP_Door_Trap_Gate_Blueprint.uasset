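; Trap gate door Blueprint that slides its mesh open and can briefly switch the player's view to a look-at camera.
; Open plays a Timeline whose track lerps the mesh from its current relative location, rather than a cached start, toward EndLocation.
; MoveCamera saves the current view target, blends to LookingCam's owner, and sets a function-name timer that blends back to the saved target.
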(event `self.ReceiveBeginPlay`)

(fn `Change camera Back`
  (bind _returnvalue (`GameplayStatics.GetActorOfClass` "/Script/Engine.PlayerController"))
  (`PlayerController.SetViewTargetWithBlend` _returnvalue (`self.Base Position`) 1.0 "VTBlend_Linear" 0.0 false))

(fn `Move Camera`
  (bind _returnvalue (`GameplayStatics.GetActorOfClass` "/Script/Engine.PlayerController"))
  (set `self.Base Position` (`Controller.GetViewTarget` _returnvalue))
  (`PlayerController.SetViewTargetWithBlend` _returnvalue (`ActorComponent.GetOwner` (`self.Looking cam`)) 1.0 "VTBlend_Linear" 0.0 false)
  (`KismetSystemLibrary.K2_SetTimer` null "Change camera Back" 3.0))

(fn `Open`
  (`TimelineComponent.Play` (`self.Timeline`)))

(fn `UserConstructionScript`)