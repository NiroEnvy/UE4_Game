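; Trigger actor that shows a dialogue phrase, plays its sound and updates the goal when the player overlaps it.
; On BeginPlay it reuses an existing top-level WB_PhrasesDisplayer widget or creates one and adds it to the viewport.
; Overlap by BP_PlayerCharacter writes the phrase and any non-empty goal into that shared widget, revealing goal text if hidden, then destroys the actor, making it single-use.
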(event `self.ReceiveBeginPlay`
  ;[1 1 1] Get ui widget
  (bind _foundwidgets (`WidgetBlueprintLibrary.GetAllWidgetsOfClass` "/Game/MyContent/Widgets/WB_PhrasesDisplayer.WB_PhrasesDisplayer_C"))
  (if (> (`KismetArrayLibrary.Array_Length` _foundwidgets) 0)
    (set `self.Widget` (`|GetArrayItem` _foundwidgets))
    (else
      (bind _returnvalue (`|CreateWidget` "/Game/MyContent/Widgets/WB_PhrasesDisplayer.WB_PhrasesDisplayer_C"))
      (bind _output_get (set `self.Widget` _returnvalue))
      (`UserWidget.AddToViewport` _output_get 0))))

(event `self.ReceiveActorBeginOverlap`
  (params (OtherActor :type "Actor Object Reference"))
  (bind _goaltext (`/Game/MyContent/Widgets/WB_PhrasesDisplayer.GoalText` (`self.Widget`)))
  ;[1 1 1] Player enters
  (if (== (`GameplayStatics.GetObjectClass` OtherActor) "/Game/FlexibleCombatSystem/Blueprints/BP_PlayerCharacter.BP_PlayerCharacter_C")
    (`|ExecutionSequence`
      (:`then_0`
        (if (not (and (`KismetTextLibrary.TextIsEmpty` (`self.Text`)) (`KismetSystemLibrary.IsValid` (`self.PhraseSound`))))
          (`GameplayStatics.PlaySound2D` (`self.PhraseSound`) 1.0 1.0 0.0 null null)
          (set `MultiLineEditableTextBox.Text` (`self.Text`) (`/Game/MyContent/Widgets/WB_PhrasesDisplayer.DialoguePhrase` (`self.Widget`)))))
      (:`then_1`
        (if (not (`KismetTextLibrary.TextIsEmpty` (`self.NewGoal`)))
          (set `MultiLineEditableTextBox.Text` (`self.NewGoal`) (`/Game/MyContent/Widgets/WB_PhrasesDisplayer.Goals` (`self.Widget`)))
          (if (not (`Widget.IsVisible` _goaltext))
            (`Widget.SetVisibility` _goaltext "Visible"))))
      (:`then_2`
        (`self.K2_DestroyActor`)))))

(fn `UserConstructionScript`)